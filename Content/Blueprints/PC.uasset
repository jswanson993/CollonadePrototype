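; PC is an actor, apparently a player character, with a swappable weapon component that defaults to bare hands and an energy-based action cooldown.
; Attack sets consumed energy from the weapon's light-attack cost, blocks acting and returns damage, while SpendEnergy adds to the total.
; Both enable Tick, which drains consumed energy, then disables itself and restores CanAct.
; OnHit's health subtraction is reversed and marked wrong, and the vulnerability check is a stub.
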(event `self.ReceiveBeginPlay`
  (bind _returnvalue (`AddComponent|NODE_AddBareHands-0`))
  (set `self.Weapon` _returnvalue))

(event `self.ReceiveTick`
  (params (DeltaSeconds :type "Float (single-precision)"))
  (if (> (`self.Energy Consumed`) 0.0)
    (bind _output_get (set `self.Energy Consumed` (- (`self.Energy Consumed`) (* DeltaSeconds (`self.Energy Recovery Rate`)))))
    (set `self.Enegry Percent Full` (/ _output_get (`self.Max Health`)))
    (else
      (`self.SetActorTickEnabled` false)
      (set `self.Can Act` true))))

(event `OnHit`
  (params (Damage :type "Float (double-precision)"))
  ;[1 1 1] This is wrong. I'm going to get to it eventually
  (bind _output_get (set `self.Max Health` (- Damage (`self.Max Health`))))
  (if (<= _output_get 0.0)
    (`self.K2_DestroyActor`)))

(fn `Attack`
  (returns (`Damage Delt` :type "Float (double-precision)"))
  (locals (`Location in Line` :type "Vector Structure" :default (0.0 0.0 0.0)))
  (bind _weapon (`self.Weapon`))
  (set `local.Location in Line` (`self.K2_GetActorLocation`))
  (`KismetSystemLibrary.PrintString` (`KismetStringLibrary.Concat_StrStr` (`KismetStringLibrary.Conv_NameToString` (`self.Name`)) " Attacks"))
  (set `self.Energy Consumed` (`/Game/Blueprints/Weapon.Light Attack Energy Cost` _weapon))
  (`self.SetActorTickEnabled` true)
  (set `self.Can Act` false)
  (return (`/Game/Blueprints/Weapon.Light Attack Damage` _weapon)))

(fn `Change Weapons`
  (params (`New Weapon` :type "/Game/Blueprints/Weapon Object Reference"))
  (`ActorComponent.K2_DestroyComponent` (`self.Weapon`))
  (set `self.Weapon` `New Weapon`))

(fn `Check Vulnerable`
  (bind _output_get (set `self.Vulnerable` false))
  (if _output_get
    (`KismetSystemLibrary.PrintString` "Vulnerable")))

(fn `Spend Energy`
  (params (Energy :type "Float (double-precision)"))
  (set `self.Energy Consumed` (+ Energy (`self.Energy Consumed`)))
  (`self.SetActorTickEnabled` true)
  (`self.Check Vulnerable`))

(fn `UserConstructionScript`)