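; Player character Blueprint with minimal, test-like logic driven by an input action named Action.
; Pressing Action prints a greeting and moves the actor to the world origin without sweeping; an unconnected vector node computes a small Y offset from its current location.
; A separate Attack function only prints the Name value with an attack message and is not called in these graphs.
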(event `InputAction|Action`
  (params (Key :type "Key Structure"))
  (:`Pressed`
    (`KismetSystemLibrary.PrintString` "Hello")
    (`self.K2_SetActorLocation` (0.0 0.0 0.0))))

(fn `Attack`
  (`KismetSystemLibrary.PrintString` (`KismetStringLibrary.Concat_StrStr` (`KismetStringLibrary.Conv_NameToString` (`self.Name`)) " Attacks")))

(fn `UserConstructionScript`)