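; Spline-travel character that detects path transition points and orients its follow camera relative to the current spline.
; Capsule overlaps store or clear the SplineTransitionPoint and, for the active character, toggle transition input on the TravelCharacterController.
; PositionCamera yaws the spring arm from the closest spline tangent, using a left or right offset chosen by the spline's camera side.
; CheckTransition and TravelState are empty, and older camera rotation code is disconnected.
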(event `self.ReceiveBeginPlay`
  (bind _astravel_character_controller (cast `/Game/Blueprints/Travel/TravelCharacterController` (`GameplayStatics.GetPlayerController` 0)))
  (set `self.playerController` _astravel_character_controller))

(event `self.CapsuleComponent.OnComponentBeginOverlap`
  (params (OverlappedComponent :type "PrimitiveComponent Object Reference") (OtherActor :type "Actor Object Reference") (OtherComp :type "PrimitiveComponent Object Reference") (OtherBodyIndex :type Integer) (bFromSweep :type Boolean) (SweepResult :type "HitResult Structure (by ref)"))
  (bind _asspline_transition_point (cast `/Game/Blueprints/Travel/SplineTransitionPoint` OtherActor))
  (set `self.TransitionPointReference` _asspline_transition_point)
  (if (`self.isActiveCharacter`)
    (bind _astravel_character_controller (cast `/Game/Blueprints/Travel/TravelCharacterController` (`GameplayStatics.GetPlayerController` 0)))
    (set `/Game/Blueprints/Travel/TravelCharacterController.transitionInputEnabled` true _astravel_character_controller)))

(event `self.CapsuleComponent.OnComponentEndOverlap`
  (params (OverlappedComponent :type "PrimitiveComponent Object Reference") (OtherActor :type "Actor Object Reference") (OtherComp :type "PrimitiveComponent Object Reference") (OtherBodyIndex :type Integer))
  (cast `/Game/Blueprints/Travel/SplineTransitionPoint` OtherActor)
  (set `self.TransitionPointReference` null)
  (if (`self.isActiveCharacter`)
    (bind _astravel_character_controller (cast `/Game/Blueprints/Travel/TravelCharacterController` (`GameplayStatics.GetPlayerController` 0)))
    (set `/Game/Blueprints/Travel/TravelCharacterController.transitionInputEnabled` false _astravel_character_controller)))

(fn `CheckTransition`)

(fn `PositionCamera`
  (bind _currentsplinereference (`/Game/Blueprints/Travel/TravelCharacterController.currentSplineReference` (`self.playerController`)))
  (if (`/Game/Blueprints/Travel/LevelSpline.IsCameraToRight` _currentsplinereference)
    (set `self.CameraYaw` (`self.RightCameraYawValue`))
    (else
      (set `self.CameraYaw` (`self.LeftCameraYawValue`))))
  (`SceneComponent.K2_SetWorldRotation` (`self.SpringArm`) (`KismetMathLibrary.ComposeRotators` (`KismetMathLibrary.Conv_VectorToRotator` (`SplineComponent.FindTangentClosestToWorldLocation` (`/Game/Blueprints/Travel/LevelSpline.Path` _currentsplinereference) (`SceneComponent.K2_GetComponentLocation` (`self.CapsuleComponent`)) "Local")) (`KismetMathLibrary.MakeRotator` 0.0 0.0 (`self.CameraYaw`))) false false))

(fn `TravelState`)

(fn `UserConstructionScript`)