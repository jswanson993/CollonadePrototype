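; Spline transition point for the travel system that switches which spline the player's TravelCharacterController references.
; TransitionUp and TransitionDown set the controller's CurrentSplineReference to the point's up or down spline and print a debug message.
; TransitionLeft and TransitionRight only print, while Reset zeroes the transition timer.
; Eligibility check, spline change, camera change and camera AI functions are empty stubs.
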(fn `ChangeCamera`)

(fn `ChangeSpline`)

(fn `CheckCanTransition`)

(fn `Reset`
  (set `self.timeToTransition` 0.0))

(fn `SetCameraAI`)

(fn `TransitionDown`
  (bind _astravel_character_controller (cast `/Game/Blueprints/Travel/TravelCharacterController` (`GameplayStatics.GetPlayerController` 0)))
  (set `/Game/Blueprints/Travel/TravelCharacterController.currentSplineReference` (`self.SplineDownReference`) _astravel_character_controller)
  (`KismetSystemLibrary.PrintString` "Transition Down"))

(fn `TransitionLeft`
  (`KismetSystemLibrary.PrintString` "Transition Left"))

(fn `TransitionRight`
  (`KismetSystemLibrary.PrintString` "Transition Right"))

(fn `TransitionUp`
  (bind _astravel_character_controller (cast `/Game/Blueprints/Travel/TravelCharacterController` (`GameplayStatics.GetPlayerController` 0)))
  (set `/Game/Blueprints/Travel/TravelCharacterController.currentSplineReference` (`self.SplineUpReference`) _astravel_character_controller)
  (`KismetSystemLibrary.PrintString` "Transition Up"))

(fn `UserConstructionScript`)