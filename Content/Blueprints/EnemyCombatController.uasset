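; Enemy combat AI controller that drives a controlled pawn through a behavior tree and supplies random targets from the party.
; On BeginPlay it caches every CharacterBP actor as the party, stores the pawn's starting location in the EnemyBB blackboard and runs EnemyBT.
; AssignTarget returns a random party entry, but passing length minus one to RandomInteger means the last entry is never picked.
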(event `self.ReceiveBeginPlay`
  (bind _outactors (`GameplayStatics.GetAllActorsOfClass` "/Game/Blueprints/CharacterBP.CharacterBP_C"))
  (set `self.Party` _outactors)
  (bind _blackboardcomponent (`self.UseBlackboard` "/Game/Blueprints/Enemy/EnemyBB.EnemyBB"))
  (`BlackboardComponent.SetValueAsVector` _blackboardcomponent (`self.Starting Location`) (`SceneComponent.K2_GetComponentLocation` (`Actor.RootComponent` (`self.K2_GetPawn`))))
  (`self.RunBehaviorTree` "/Game/Blueprints/Enemy/EnemyBT.EnemyBT"))

(fn `Assign Target`
  (returns (`New Target` :type "/Game/Blueprints/CharacterBP Object Reference"))
  (locals (`Targeted Character` :type Name :default "Targeted Character"))
  (return (`|GetArrayItem` (`self.Party`) (`KismetMathLibrary.RandomInteger` (- (`KismetArrayLibrary.Array_Length` (`self.Party`)) 1)))))

(fn `UserConstructionScript`)