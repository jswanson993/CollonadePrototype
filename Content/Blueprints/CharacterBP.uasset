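; Combat character Blueprint that attacks with a weapon component, tracks damage and energy spent, and starts with bare hands.
; Attacks set energy cost and block acting; Tick drains it at a recovery rate, then disables itself and restores acting.
; Blocked hits convert damage into energy spent, while lethal damage hides the actor and notifies PlayerCombatController of an enemy death.
; OnHit is flagged as wrong, and the vulnerability check is stubbed.
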(event `self.ReceiveBeginPlay`
  (bind _returnvalue (`AddComponent|NODE_AddBareHands-0`))
  (set `self.Weapon_Depricated` _returnvalue))

(event `self.ReceiveTick`
  (params (DeltaSeconds :type "Float (single-precision)"))
  (if (> (`self.Energy Consumed`) 0.0)
    (bind _output_get (set `self.Energy Consumed` (- (`self.Energy Consumed`) (* DeltaSeconds (`self.Energy Recovery Rate`)))))
    (set `self.Enegry Percent Full` (/ _output_get (`self.Max Health`)))
    (else
      (set `self.Energy Consumed` 0.0)
      (`self.SetActorTickEnabled` false)
      (set `self.Can Act` true))))

(event `OnHit`
  (params (Damage :type "Float (double-precision)"))
  ;[1 1 1] This is wrong. I'm going to get to it eventually
  (bind _output_get (set `self.Max Health` (- Damage (`self.Max Health`))))
  (if (<= _output_get 0.0)
    (`self.K2_DestroyActor`)))

(event `Dead`
  (`self.SetActorHiddenInGame` true)
  (bind _asplayer_combat_controller (cast `/Game/Blueprints/Controllers/PlayerCombatController` (`GameplayStatics.GetPlayerController` 0)))
  (`/Game/Blueprints/Controllers/PlayerCombatController.EnemyDead` _asplayer_combat_controller))

(fn `Attack`
  (returns (`Damage Delt` :type "Float (double-precision)"))
  (locals (`Location in Line` :type "Vector Structure" :default (0.0 0.0 0.0)))
  (bind _weapon_depricated (`self.Weapon_Depricated`))
  (set `local.Location in Line` (`self.K2_GetActorLocation`))
  (`KismetSystemLibrary.PrintString` (`KismetStringLibrary.Concat_StrStr` (`KismetStringLibrary.Conv_NameToString` (`self.Name`)) " Attacks"))
  (set `self.Energy Consumed` (`/Game/Blueprints/Weapon_Depricated.Light Attack Energy Cost` _weapon_depricated))
  (set `self.Can Act` false)
  (return (`/Game/Blueprints/Weapon_Depricated.Light Attack Damage` _weapon_depricated)))

(fn `Attacking`
  (params (`Is Attacking` :type Boolean))
  (`self.SetActorTickEnabled` (not `Is Attacking`)))

(fn `Change Weapons`
  (params (`New Weapon` :type "/Game/Blueprints/Weapon_Depricated Object Reference"))
  (`ActorComponent.K2_DestroyComponent` (`self.Weapon_Depricated`))
  (set `self.Weapon_Depricated` `New Weapon`))

(fn `Check Vulnerable`
  (bind _output_get (set `self.Vulnerable` false))
  (if _output_get
    (`KismetSystemLibrary.PrintString` "Vulnerable")))

(fn `Spend Energy`
  (params (Energy :type "Float (double-precision)"))
  (set `self.Energy Consumed` (+ Energy (`self.Energy Consumed`)))
  (`self.SetActorTickEnabled` true)
  (`self.Check Vulnerable`))

(fn `Take Damage`
  (params (Damage :type "Float (double-precision)"))
  (locals (`Actual Damage Taken` :type "Float (double-precision)"))
  (bind _max_health (`self.Max Health`))
  (if (`self.Blocked`)
    (`KismetSystemLibrary.PrintString` "Blocked")
    (`self.Spend Energy` Damage)
    (`self.SetActorTickEnabled` true)
    (set `local.Actual Damage Taken` 0.0)
    (else
      (set `local.Actual Damage Taken` Damage)))
  (`KismetSystemLibrary.PrintString` (`KismetStringLibrary.Concat_StrStr` (`KismetSystemLibrary.GetDisplayName` self) "Takes" (`KismetStringLibrary.Conv_DoubleToString` (`local.Actual Damage Taken`)) "Damage"))
  (bind _output_get (set `self.Damage Taken` (+ (`self.Damage Taken`) (`local.Actual Damage Taken`))))
  (set `self.Damage Percent Full` (/ _output_get _max_health))
  (if (>= _output_get _max_health)
    (`self.Dead`)))

(fn `Take Damage Passives`)

(fn `UserConstructionScript`)