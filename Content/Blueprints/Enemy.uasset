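; Enemy Blueprint that tracks health, spent energy and a vulnerable state.
; TakeDamage prints the hit, subtracts it directly from MaxHealth and returns whether health is depleted.
; SpendEnergy accumulates EnergyConsumed, and CheckVulnerable sets Vulnerable when that plus DamageTaken exceeds MaxHealth, though nothing here updates DamageTaken.
; The Dead event only binds itself to the EventDead dispatcher, and Tick is empty.
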(event `self.ReceiveTick`
  (params (DeltaSeconds :type "Float (single-precision)")))

(event `Dead`
  (add `self.Event_Dead` (delegate `Dead`)))

(fn `Check Vulnerable`
  (set `self.Vulnerable` (> (+ (`self.Damage Taken`) (`self.Energy Consumed`)) (`self.Max Health`))))

(fn `Spend Energy`
  (params (Energy :type "Float (double-precision)"))
  (set `self.Energy Consumed` (+ Energy (`self.Energy Consumed`))))

(fn `TakeDamage`
  (params (Damage :type "Float (double-precision)"))
  (returns (Dead :type Boolean))
  (`KismetSystemLibrary.PrintString` (`KismetStringLibrary.Concat_StrStr` (`KismetSystemLibrary.GetDisplayName` self) "Takes" (`KismetStringLibrary.Conv_DoubleToString` Damage) "Damage"))
  (bind _output_get (set `self.Max Health` (- (`self.Max Health`) Damage)))
  (return (<= _output_get 0.0)))

(fn `UserConstructionScript`)