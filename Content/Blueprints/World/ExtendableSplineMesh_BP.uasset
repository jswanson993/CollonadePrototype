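; A world-building Blueprint that tiles a mesh along an editable spline as blocking, collidable spline mesh segments.
; The construction script splits the spline into a set segment count, or one derived from its length, and adds a component per segment with optional material override.
; Each piece overlaps its neighbours by a percentage, takes a vertical offset, and uses normalised tangents scaled by segment length, capped by a tuning value.
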(fn `UserConstructionScript`
  (locals (index :type Integer) (lengthPerMesh :type "Float (double-precision)"))
  (bind _lengthpermesh (`local.lengthPerMesh`))
  (bind _spline (`self.Spline`))
  (bind _lengthpermesh_2 (`local.lengthPerMesh`))
  (bind _returnvalue (`SplineComponent.GetSplineLength` (`self.Spline`)))
  (bind _returnvalue_2 (* (0.0 0.0 1.0) (`self.MeshVerticalOffset`)))
  (bind _returnvalue_3 (`KismetMathLibrary.FClamp` (`local.lengthPerMesh`) 0.0 (`self.TangentTuning`)))
  (bind _returnvalue_4 (- (* (`local.index`) _lengthpermesh_2) (* _lengthpermesh_2 (`self.PercentageOverlap`))))
  (bind _returnvalue_5 (+ (* (+ (`local.index`) 1) _lengthpermesh) (* _lengthpermesh (`self.PercentageOverlap`))))
  (if (`self.AutoSegments`)
    (set `self.Segments` (`KismetMathLibrary.Round` (/ _returnvalue (`self.LengthPerAutoSegment`)))))
  (set `local.lengthPerMesh` (/ _returnvalue (`KismetMathLibrary.Conv_IntToDouble` (`self.Segments`))))
  (for _index (range (`self.Segments`))
    (set `local.index` _index)
    (bind _returnvalue_6 (`AddComponent|NODE_AddSplineMeshComponent-0`))
    (`|ExecutionSequence`
      (:`then_0`
        (`StaticMeshComponent.SetStaticMesh` _returnvalue_6 (`self.Mesh`))
        (`SplineMeshComponent.SetForwardAxis` _returnvalue_6 (`self.ForwardAxis`) true)
        (`PrimitiveComponent.SetCollisionEnabled` _returnvalue_6 "QueryAndPhysics")
        (`PrimitiveComponent.SetCollisionProfileName` _returnvalue_6 "BlockAll" true)
        (set `PrimitiveComponent.bGenerateOverlapEvents` true _returnvalue_6)
        (`PrimitiveComponent.SetCollisionObjectType` _returnvalue_6 "ECC_WorldStatic")
        (`PrimitiveComponent.SetNotifyRigidBodyCollision` _returnvalue_6 true)
        (if (`self.Override Material`)
          (`PrimitiveComponent.SetMaterial` _returnvalue_6 0 (`self.Material`))))
      (:`then_1`
        (`SplineMeshComponent.SetStartAndEnd` _returnvalue_6 (+ _returnvalue_2 (`SplineComponent.GetLocationAtDistanceAlongSpline` _spline _returnvalue_4 "Local")) (* (`KismetMathLibrary.Vector_NormalUnsafe` (`SplineComponent.GetTangentAtDistanceAlongSpline` _spline _returnvalue_4 "Local")) _returnvalue_3) (+ _returnvalue_2 (`SplineComponent.GetLocationAtDistanceAlongSpline` _spline _returnvalue_5 "Local")) (* (`KismetMathLibrary.Vector_NormalUnsafe` (`SplineComponent.GetTangentAtDistanceAlongSpline` _spline _returnvalue_5 "Local")) _returnvalue_3) true)))))