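; WaterGrid_BP lays out a grid of mesh tiles, named as a water surface, from configurable row and column counts.
; The construction script assigns the mesh to a Hierarchical Instanced Static Mesh component and adds one instance per cell at a fixed spacing.
; It disables shadow casting and can optionally override the material.
; The event graph is empty, so the actor has no runtime logic of its own.
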(fn `UserConstructionScript`
  (bind _hierarchicalinstancedstaticmesh (`self.HierarchicalInstancedStaticMesh`))
  (`StaticMeshComponent.SetStaticMesh` (`self.HierarchicalInstancedStaticMesh`) (`self.Mesh`))
  (for _index (range (`self.rows`))
    (for _index_2 (range (`self.cols`))
      (`InstancedStaticMeshComponent.AddInstance` _hierarchicalinstancedstaticmesh (`KismetMathLibrary.MakeTransform` (`KismetMathLibrary.MakeVector` (* _index_2 1000.0) (* _index 1000.0))))
      (`PrimitiveComponent.SetCastShadow` _hierarchicalinstancedstaticmesh false)
      (if (`self.OverrideMaterial`)
        (`PrimitiveComponent.SetMaterial` _hierarchicalinstancedstaticmesh 0 (`self.Material`))))))