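; BattleManager coordinates attack turns between party and enemy characters, merging both lists into one on BeginPlay.
; When a character attacks, it disables every other character's ability to act and freezes them with zero CustomTimeDilation, restoring all when the attack finishes.
; It also relays attack window start and end through event dispatchers and provides a function to clear party members' Blocked flags.
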(event `Event Character Attacking`
  (params (Character :type "Pawn Object Reference"))
  (bind _output_get (set `self.Attacking Character` Character))
  (for _array_element (`self.All Characters`)
    (if (not (== _output_get _array_element))
      (set `/Game/Blueprints/CharacterBP.Can Act` false _array_element)
      (set `Actor.CustomTimeDilation` 0.0 _array_element))))

(event `Attack Finished`
  (for _array_element (`self.All Characters`)
    (set `Actor.CustomTimeDilation` 1.0 _array_element)
    (set `/Game/Blueprints/CharacterBP.Can Act` true _array_element)))

(event `self.ReceiveBeginPlay`
  (bind _all_characters (`self.All Characters`))
  (`KismetArrayLibrary.Array_Append` _all_characters (`self.Party`))
  (`KismetArrayLibrary.Array_Append` _all_characters (`self.Enemy Characters`)))

(event `Attack Window Starting`
  (`self.Attack Window Start Dispatch`))

(event `Attack Window Ending`
  (`self.Attack Window End Dispatch`))

(fn `Reset Blocks`
  (for _array_element (`self.Party`)
    (set `/Game/Blueprints/CharacterBP.Blocked` false _array_element)))

(fn `UserConstructionScript`)