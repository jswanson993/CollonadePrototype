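; Enemy Blueprint for combat that holds health, energy use and vulnerability state.
; TakeDamage prints a debug message, subtracts damage directly from MaxHealth and fires Dead at zero or below, which notifies the PlayerCombatController.
; SpendEnergy accumulates EnergyConsumed, and CheckVulnerable sets Vulnerable when that plus DamageTaken exceeds MaxHealth.
; DamageTaken is not updated here, and a comment suggests damage handling may move to an enemy controller.
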(event `self.ReceiveTick`
  (params (DeltaSeconds :type "Float (single-precision)")))

(event `Dead`
  (bind _asplayer_combat_controller (cast `/Game/Blueprints/PlayerCombatController` (`GameplayStatics.GetPlayerController` 0)))
  (`/Game/Blueprints/PlayerCombatController.EnemyDead` _asplayer_combat_controller))

(fn `Check Vulnerable`
  (set `self.Vulnerable` (> (+ (`self.Damage Taken`) (`self.Energy Consumed`)) (`self.Max Health`))))

(fn `Spend Energy`
  (params (Energy :type "Float (double-precision)"))
  (set `self.Energy Consumed` (+ Energy (`self.Energy Consumed`))))

(fn `TakeDamage`
  (params (Damage :type "Float (double-precision)"))
  ;[1 1 1] Maybe move this to enemy controller once implemented?
  (`KismetSystemLibrary.PrintString` (`KismetStringLibrary.Concat_StrStr` (`KismetSystemLibrary.GetDisplayName` self) "Takes" (`KismetStringLibrary.Conv_DoubleToString` Damage) "Damage"))
  (bind _output_get (set `self.Max Health` (- (`self.Max Health`) Damage)))
  (if (<= _output_get 0.0)
    (`self.Dead`)))

(fn `UserConstructionScript`)