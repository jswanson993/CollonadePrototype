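; Player combat controller that lets the player pick one of four party members and attack a focused enemy.
; BeginPlay gathers all PC and Enemy actors; four input actions set the active character, and D-pad left/right moves enemy focus.
; Action repeats the character's attack per its weapon's light attack count, hiding and removing killed enemies, refocusing, and quitting when none remain.
; SelectCharacter is unused, and LightAttack duplicates the attack loop without death handling.
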(event `self.ReceiveBeginPlay`
  (bind _outactors (`GameplayStatics.GetAllActorsOfClass` "/Game/Blueprints/PC.PC_C"))
  (set `self.Party` _outactors)
  (bind _outactors_2 (`GameplayStatics.GetAllActorsOfClass` "/Game/Blueprints/Enemy.Enemy_C"))
  (bind _output_get (set `self.Enemies` _outactors_2))
  (set `self.Focused Enemy` (`|GetArrayItem` _output_get (`self.EnemyID`))))

(event `self.ReceiveTick`
  (params (DeltaSeconds :type "Float (single-precision)")))

(event `InputAction|Outer Left`
  (params (Key :type "Key Structure"))
  ;[1 1 1] Select which characters are being controlled
  (:`Pressed`
    (set `self.Selected Character` 0)))

(event `InputAction|Inner Left`
  (params (Key :type "Key Structure"))
  ;[1 1 1] Select which characters are being controlled
  (:`Pressed`
    (set `self.Selected Character` 1)))

(event `InputAction|Inner Right`
  (params (Key :type "Key Structure"))
  ;[1 1 1] Select which characters are being controlled
  (:`Pressed`
    (set `self.Selected Character` 2)))

(event `InputAction|Outer Right`
  (params (Key :type "Key Structure"))
  ;[1 1 1] Select which characters are being controlled
  (:`Pressed`
    (set `self.Selected Character` 3)))

(event `InputAction|Action`
  (params (Key :type "Key Structure"))
  (bind _returnvalue (`KismetArrayLibrary.Array_Length` (`self.Enemies`)))
  ;[1 1 1] When attack button is hit go through active characters and attack target
  (:`Pressed`
    (bind _aspc (cast `/Game/Blueprints/PC` (`|GetArrayItem` (`self.Party`) (`self.Selected Character`))))
    (if (`/Game/Blueprints/PC.Can Act` _aspc)
      (for _ (range (`/Game/Blueprints/Weapon.Light Attack Num` (`/Game/Blueprints/PC.Weapon` _aspc)))
        (bind _damage_delt (`/Game/Blueprints/PC.Attack` _aspc))
        (bind _dead (`/Game/Blueprints/Enemy.TakeDamage` (`self.Focused Enemy`) _damage_delt))
        ;[1 1 1] If enemy is killed, hide them and fucus on next enemy
        (if _dead
          (`SceneComponent.SetVisibility` (`/Game/Blueprints/Enemy.DefaultSceneRoot` (`self.Focused Enemy`)) false true)
          (`KismetArrayLibrary.Array_Remove` (`self.Enemies`) (`self.EnemyID`))
          ;[1 0.1506 0.9505] When all enemies are defeated quit game (change later)
          (if (== (`KismetArrayLibrary.Array_Length` (`self.Enemies`)) 0)
            (`KismetSystemLibrary.QuitGame` null "Quit")
            (else
              (if (>= (`self.EnemyID`) _returnvalue)
                (set `self.EnemyID` (- _returnvalue 1)))
              (set `self.Focused Enemy` (`|GetArrayItem` (`self.Enemies`) (`self.EnemyID`))))))))))

(event `Key|Gamepad_DPad_Left`
  (params (Key :type "Key Structure"))
  (bind _returnvalue (- (`self.EnemyID`) 1))
  ;[1 1 1] Set which enemy is selected based of dpad input. May change to different input
  (:`Pressed`
    (if (>= _returnvalue 0) :!label _label
      (bind _output_get (set `self.EnemyID` _returnvalue))
      (bind _output (`|GetArrayItem` (`self.Enemies`) _output_get))
      (`/Engine/EditorBlueprintResources/StandardMacros.IsValid` _output
        (:`Is Valid`
          (set `self.Focused Enemy` _output))
        (:`Is Not Valid`
          (goto _label))))))

(event `Key|Gamepad_DPad_Right`
  (params (Key :type "Key Structure"))
  (bind _returnvalue (+ (`self.EnemyID`) 1))
  ;[1 1 1] Set which enemy is selected based of dpad input. May change to different input
  (:`Pressed`
    (if (<= _returnvalue (`KismetArrayLibrary.Array_Length` (`self.Enemies`))) :!label _label_2
      (bind _output_get (set `self.EnemyID` _returnvalue))
      (bind _output (`|GetArrayItem` (`self.Enemies`) _output_get))
      (`/Engine/EditorBlueprintResources/StandardMacros.IsValid` _output
        (:`Is Valid`
          (set `self.Focused Enemy` _output))
        (:`Is Not Valid`
          (goto _label_2))))))

(fn `Light Attack`
  (bind _aspc (cast `/Game/Blueprints/PC` (`|GetArrayItem` (`self.Party`) (`self.Selected Character`))))
  (if (`/Game/Blueprints/PC.Can Act` _aspc)
    (for _ (range (`/Game/Blueprints/Weapon.Light Attack Num` (`/Game/Blueprints/PC.Weapon` _aspc)))
      (bind _damage_delt (`/Game/Blueprints/PC.Attack` _aspc))
      (`/Game/Blueprints/Enemy.TakeDamage` (`self.Focused Enemy`) _damage_delt))))

(fn `Select Character`
  (params (CharacterID :type Integer) (IsSelecting :type Boolean))
  ;[1 0 0.0648] No longer being used. Keeping in case we change how characters are selected
  (`KismetSystemLibrary.PrintString` (`KismetStringLibrary.Conv_IntToString` CharacterID))
  (`KismetArrayLibrary.Array_Set` (`self.Selected Characters`) 0 IsSelecting))

(fn `UserConstructionScript`)