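; Design-time combat simulator that runs repeated fights against one enemy on BeginPlay and prints how many ticks each kill takes.
; Each tick either attacks once fatigue reaches zero, adding the attack's cost, or recovers fatigue.
; Attacks subtract armor from damage and roll for a bonus: chance-based extra hits or added damage, with an optional fatigue refund.
; A loop for multiple base attacks is left disconnected.
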(event `self.ReceiveBeginPlay`
  (set `self.startingEnemyHealth` (`self.EnemyHealth`))
  (for _ (range 51)
    (set `self.EnemyHealth` (`self.startingEnemyHealth`))
    (if (`self.isNewFight`)
      (set `self.NumTicks` 0)
      (set `self.isNewFight` false)
      (set `self.CurrentFatigue` (`self.StartingFatigue`)))
    (while (> (`self.EnemyHealth`) 0)
      (if (<= (`self.CurrentFatigue`) 0)
        ;[1 1 1] IncreaseFatigue
        (set `self.CurrentFatigue` (`KismetMathLibrary.Clamp` (+ (`self.CurrentFatigue`) (`self.AttackCost`)) 0 (`self.MaxFatigue`)))
        (set `self.isAttacking` true)
        ;[1 1 1] Make an attack with chance for bonus
        (if (<= (`KismetMathLibrary.RandomFloatInRange` 0.0 100.0) (`self.ChanceForBonus`))
          (set `self.BonusTriggered` true)
          ;[1 1 1] Calculating Number of Gated Bonus Attacks
          (if (`self.BonusIsExtraAttack`)
            (set `self.bonusAttacks` 0)
            (for _ (range 1 (+ (`self.numMaxPossibleBonusAttacks`) 1))
              (if (<= (`KismetMathLibrary.RandomFloatInRange` 0.0 100.0) (`self.ChanceForBonus`))
                (`/Engine/EditorBlueprintResources/StandardMacros.IncrementInt` (`self.bonusAttacks`))))
            ;[1 1 1] Damage for All Succesful Bonus Attacks
            (for _ (range (+ (`self.bonusAttacks`) 1))
              (set `self.EnemyHealth` (- (`self.EnemyHealth`) (- (`self.AttackDamage`) (`self.EnemyArmor`)))))
            (else
              ;[1 1 1] Single Attack With Bonus Damage
              (set `self.EnemyHealth` (- (`self.EnemyHealth`) (- (+ (`self.AttackDamage`) (`self.BonusDamage`)) (`self.EnemyArmor`))))))
          (else
            ;[1 1 1] Single Attack With no Bonus
            (set `self.EnemyHealth` (- (`self.EnemyHealth`) (- (`self.AttackDamage`) (`self.EnemyArmor`))))))
        (set `self.isAttacking` false)
        ;[1 1 1] Refund Fatigue if that is the Bonus
        (if (and (`self.BonusIsFatigueRefund`) (`self.BonusTriggered`))
          (set `self.BonusTriggered` false)
          (set `self.CurrentFatigue` (- (`self.CurrentFatigue`) (`self.FatigueRefundAmmount`)))
          (else
            (set `self.BonusTriggered` false)))
        ;[1 1 1] Increase Second Count
        (`/Engine/EditorBlueprintResources/StandardMacros.IncrementInt` (`self.NumTicks`) :!label _label
          (:`  `
            ;[1 1 1] End Loop and Print Num Seconds
            (if (<= (`self.EnemyHealth`) 0)
              (`KismetSystemLibrary.PrintString` (`KismetStringLibrary.Conv_IntToString` (`self.NumTicks`)) true true (struct :`G` 0.66 :`B` 1.0 :`A` 1.0) 10.0)
              (set `self.isNewFight` true))))
        (elif (not (`self.isAttacking`))
          ;[1 1 1] Regen Energy If Can't Attack
          (set `self.CurrentFatigue` (`KismetMathLibrary.Clamp` (- (`self.CurrentFatigue`) (`self.EnergyRegen`)) 0 (`self.MaxFatigue`)))
          (goto _label))))))

(fn `UserConstructionScript`)