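; Player controller for party-based combat that lets one player command several characters against a shared list of enemies.
; It reads Party and Enemies from the controlled PlayerView pawn, with four inputs selecting a character and D-pad left/right cycling its target.
; The action input delegates a light attack to the selected character's AI CombatController.
; Enemy death removes the focused index, retargets party members on that enemy, and quits the game when none remain.
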(event `self.ReceiveBeginPlay`
  (add `self.EnemyDead` (delegate `Enemy Killed`))
  (bind _asplayer_view (cast `/Game/Blueprints/PlayerView` (`self.K2_GetPawn`)))
  (set `self.Party` (`/Game/Blueprints/PlayerView.Party` _asplayer_view))
  (bind _output_get (set `self.Enemies` (`/Game/Blueprints/PlayerView.Enemies` _asplayer_view)))
  (set `self.Focused Enemy` (`|GetArrayItem` _output_get (`self.EnemyID`)))
  (for _array_element (`self.Party`)
    (set `/Game/Blueprints/CharacterBP.Targeting` (`self.Focused Enemy`) _array_element))
  (bind _returnvalue (`GameplayStatics.GetActorOfClass` "/Game/Blueprints/BattleManager.BattleManager_C"))
  (set `self.Battle Manager` _returnvalue))

(event `Enemy Killed`
  (`self.Remove Enemy`))

(event `self.ReceiveTick`
  (params (DeltaSeconds :type "Float (single-precision)")))

(event `InputAction|Outer Left`
  (params (Key :type "Key Structure"))
  ;[1 1 1] Select which characters are being controlled
  (:`Pressed`
    (`self.Select Character` 0)))

(event `InputAction|Inner Left`
  (params (Key :type "Key Structure"))
  ;[1 1 1] Select which characters are being controlled
  (:`Pressed`
    (`self.Select Character` 1)))

(event `InputAction|Inner Right`
  (params (Key :type "Key Structure"))
  ;[1 1 1] Select which characters are being controlled
  (:`Pressed`
    (`self.Select Character` 2)))

(event `InputAction|Outer Right`
  (params (Key :type "Key Structure"))
  ;[1 1 1] Select which characters are being controlled
  (:`Pressed`
    (`self.Select Character` 3)))

(event `InputAction|Action`
  (params (Key :type "Key Structure"))
  (:`Pressed`
    (`self.Light Attack`)))

(event `Key|Gamepad_DPad_Left`
  (params (Key :type "Key Structure"))
  (bind _returnvalue (- (`self.EnemyID`) 1))
  ;[1 1 1] Set which enemy is selected based of dpad input. May change to different input
  (:`Pressed`
    (if (>= _returnvalue 0) :!label _label
      (bind _output_get (set `self.EnemyID` _returnvalue))
      (bind _output (`|GetArrayItem` (`self.Enemies`) _output_get))
      (`/Engine/EditorBlueprintResources/StandardMacros.IsValid` _output
        (:`Is Valid`
          (set `self.Focused Enemy` _output)
          (set `/Game/Blueprints/CharacterBP.Targeting` (`self.Focused Enemy`) (`self.Selected Character`) :!label _label_2))
        (:`Is Not Valid`
          (goto _label))))))

(event `Key|Gamepad_DPad_Right`
  (params (Key :type "Key Structure"))
  (bind _returnvalue (+ (`self.EnemyID`) 1))
  ;[1 1 1] Set which enemy is selected based of dpad input. May change to different input
  (:`Pressed`
    (if (<= _returnvalue (`KismetArrayLibrary.Array_Length` (`self.Enemies`))) :!label _label_3
      (bind _output_get (set `self.EnemyID` _returnvalue))
      (bind _output (`|GetArrayItem` (`self.Enemies`) _output_get))
      (`/Engine/EditorBlueprintResources/StandardMacros.IsValid` _output
        (:`Is Valid`
          (set `self.Focused Enemy` _output)
          (goto _label_2))
        (:`Is Not Valid`
          (goto _label_3))))))

(fn `Light Attack`
  (locals (`Attacking Character` :type "/Game/Blueprints/CharacterBP Object Reference"))
  (bind _ascombat_controller (cast `/Game/Blueprints/Controllers/CombatController` (`AIBlueprintHelperLibrary.GetAIController` (`self.Selected Character`))))
  (`/Game/Blueprints/Controllers/CombatController.Attack` _ascombat_controller))

(fn `Remove Enemy`
  (bind _returnvalue (`KismetArrayLibrary.Array_Length` (`self.Enemies`)))
  (bind _output (`|GetArrayItem` (`self.Enemies`) (`self.EnemyID`)))
  ;[1 1 1] If enemy is killed, hide them and focus on next enemy
  (`KismetArrayLibrary.Array_Remove` (`self.Enemies`) (`self.EnemyID`))
  ;[1 0.1506 0.9505] When all enemies are defeated quit game (change later) Maybe move to game instance
  (if (== (`KismetArrayLibrary.Array_Length` (`self.Enemies`)) 0)
    (`KismetSystemLibrary.QuitGame` null "Quit")
    (else
      (if (>= (`self.EnemyID`) _returnvalue)
        (set `self.EnemyID` (- _returnvalue 1)))
      ;;[0.3231 0.2395 1] If any other player is targeting the same enemy change their target
      (for _array_element (`self.Party`)
        (if (== (`/Game/Blueprints/CharacterBP.Targeting` _array_element) (`self.Focused Enemy`))
          (set `/Game/Blueprints/CharacterBP.Targeting` _output _array_element)))
      (set `self.Focused Enemy` _output))))

(fn `Select Character`
  (params (CharacterID :type Integer))
  (if (< CharacterID (`KismetArrayLibrary.Array_Length` (`self.Party`)))
    (bind _output_get (set `self.Selected Character` (`|GetArrayItem` (`self.Party`) CharacterID)))
    (bind _asenemy_bp (cast `/Game/Blueprints/Enemy_BP` (`/Game/Blueprints/CharacterBP.Targeting` _output_get)))
    (set `self.Focused Enemy` _asenemy_bp)))

(fn `UserConstructionScript`)