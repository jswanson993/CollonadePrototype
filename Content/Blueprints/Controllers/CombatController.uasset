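; CombatController is a controller that runs a pawn's melee attack in battle, starting from and returning to a stored battle-line position.
; Attack notifies the BattleManager if the character can act, then uses AI MoveTo to reach its target.
; It applies one hit per weapon light-attack count, moves back, then reports the attack finished.
; Behavior tree setup and an older move sequence remain unconnected.
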(event `self.ReceiveBeginPlay`
  (bind _output_get (set `self.Controlled Pawn` (`self.K2_GetPawn`)))
  (set `self.Battle Line Location` (`self.K2_GetActorLocation` _output_get))
  (bind _returnvalue (`GameplayStatics.GetActorOfClass` "/Game/Blueprints/BattleManager.BattleManager_C"))
  (set `self.Battle Manager` _returnvalue))

(event `Attack`
  (bind _attacking_character (`self.Attacking Character`))
  (bind _attacking_character_2 (`self.Attacking Character`))
  ;[1 1 1] This would likely change depending on the type of weapon
  (bind _ascharacter_bp (cast `/Game/Blueprints/CharacterBP` (`self.Controlled Pawn`)))
  (bind _output_get (set `self.Attacking Character` _ascharacter_bp))
  (if (`/Game/Blueprints/CharacterBP.Can Act` _ascharacter_bp)
    (`/Game/Blueprints/BattleManager.Event Character Attacking` (`self.Battle Manager`) (`self.Attacking Character`))
    ;;[1 0 0] This started failing out of nowhere and I have no idea why
    (`|AIMoveTo` _attacking_character (0.0 0.0 0.0) (`/Game/Blueprints/CharacterBP.Targeting` _attacking_character) 0.0
      (:`OnSuccess`
        (for _ (range (`/Game/Blueprints/Weapon.Light Attack Num` (`/Game/Blueprints/CharacterBP.Weapon` _output_get)))
          (bind _damage_delt (`/Game/Blueprints/CharacterBP.Attack` _attacking_character_2))
          (`/Game/Blueprints/CharacterBP.Take Damage` (`/Game/Blueprints/CharacterBP.Targeting` _attacking_character_2) _damage_delt))
        (`|AIMoveTo` (`self.Attacking Character`) (`self.Battle Line Location`) null 0.5
          (:`OnSuccess`
            (`/Game/Blueprints/BattleManager.Attack Finished` (`self.Battle Manager`)))
          (:`OnFail`
            _))
        (`KismetSystemLibrary.PrintString` "Hello")))))

(fn `UserConstructionScript`)