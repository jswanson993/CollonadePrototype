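; PlayerView manages the party's health and energy HUD and the highlighting of targeted characters.
; On BeginPlay it creates one CharacterHealthAndEnergy widget per Party member, spaced at quarter intervals of a hardcoded 1920-pixel width.
; UpdateHealth and UpdateEnergy set paired progress bars in the widget indexed by CharacterID.
; SetTargets clears the previous targets' custom depth rendering, then enables it on the new targets' meshes as a highlight.
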(event `self.ReceiveBeginPlay`
  (for (_array_element _array_index) (`self.Party`)
    (bind _returnvalue (`|CreateWidget` "/Game/Widgets/CharacterHealthAndEnergy.CharacterHealthAndEnergy_C" (`GameplayStatics.GetPlayerController` 0) _array_element))
    (`KismetArrayLibrary.Array_Add` (`self.Party Bars`) _returnvalue)
    (`Widget.SetRenderTranslation` _returnvalue (`KismetMathLibrary.MakeVector2D` (* (+ _array_index 0) (* 1920.0 0.25)) -50.0))
    (`UserWidget.AddToViewport` _returnvalue 0)))

(event `Update Health`
  (params (`health  percentage` :type "Float (double-precision)") (`Character ID` :type Integer))
  (`ProgressBar.SetPercent` (`/Game/Widgets/CharacterHealthAndEnergy.DamageTaken` (`|GetArrayItem` (`self.Party Bars`) `Character ID`)) `health  percentage`)
  (`ProgressBar.SetPercent` (`/Game/Widgets/CharacterHealthAndEnergy.Damage` (`|GetArrayItem` (`self.Party Bars`) `Character ID`)) `health  percentage`))

(event `Update Energy`
  (params (`energy percentage` :type "Float (double-precision)") (`Character ID` :type Integer))
  (`ProgressBar.SetPercent` (`/Game/Widgets/CharacterHealthAndEnergy.EnergyConsumption` (`|GetArrayItem` (`self.Party Bars`) `Character ID`)) `energy percentage`)
  (`ProgressBar.SetPercent` (`/Game/Widgets/CharacterHealthAndEnergy.Energy` (`|GetArrayItem` (`self.Party Bars`) `Character ID`)) `energy percentage`))

(fn `Highlight`
  (for _array_element (`self.Targets`)
    (`PrimitiveComponent.SetRenderCustomDepth` (`Character.Mesh` _array_element) true)))

(fn `SetTargets`
  (params (`Target Characters` :type "Array of /Game/Blueprints/CharacterBP Object Reference"))
  (`self.Stop Targeting`)
  (set `self.Targets` `Target Characters`)
  (`self.Highlight`))

(fn `Stop Targeting`
  (for _array_element (`self.Targets`)
    (if (`KismetSystemLibrary.IsValid` _array_element)
      (`PrimitiveComponent.SetRenderCustomDepth` (`Character.Mesh` _array_element) false))))

(fn `UserConstructionScript`)